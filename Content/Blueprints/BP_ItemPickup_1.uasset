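; BP_ItemPickup_1 is an interactable key pickup that advances a collection quest objective when the player picks it up.
; It always allows interaction and shows an "E — Pick Up Key" prompt.
; Interact finds the first QuestComponent on the interactor, adds progress to the hardcoded Collect1 objective, then destroys the pickup.
; An interactor without a QuestComponent leaves it in place.
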(event `InteractionInterface.Interact`
  (params (Interactor :type "Actor Object Reference"))
  (bind _returnvalue (`self.K2_GetComponentsByClass` Interactor "/Script/InteractionToolkit.QuestComponent"))
  (if (> (`KismetArrayLibrary.Array_Length` _returnvalue) 0)
    (`QuestComponent.UpdateProgress` (`|GetArrayItem` _returnvalue) "Collect1" 1)
    (`self.K2_DestroyActor`)))

(fn `CanInteract`
  (params (Interactor :type "Actor Object Reference"))
  (returns (ReturnValue :type Boolean))
  (return true))

(fn `GetInteractionText`
  (returns (ReturnValue :type Text))
  (return "E — Pick Up Key"))

(fn `UserConstructionScript`)